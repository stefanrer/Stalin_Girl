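; NormTalkableChar is an interactable character that plays a black-screen transition when the player presses E nearby, with no dialogue logic yet.
; Player overlap toggles the actor's input, and E disables pawn input and adds a new BlackScreen widget.
; The player's side on the X axis selects the Right or Left timeline, which drives widget opacity and restores pawn input when finished.
; Flipbook rotation nodes are left unwired.
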(event `self.ReceiveActorEndOverlap`
  (params (OtherActor :type "Actor Object Reference"))
  (cast `/Game/PlayerCharacter/PlayerCharacter` OtherActor)
  (`self.DisableInput` (`GameplayStatics.GetPlayerController` 0)))

(event `self.ReceiveActorBeginOverlap`
  (params (OtherActor :type "Actor Object Reference"))
  (bind _asplayer_character (cast `/Game/PlayerCharacter/PlayerCharacter` OtherActor))
  (`self.EnableInput` (`GameplayStatics.GetPlayerController` 0)))

(event `Key|E`
  (params (Key :type "Key Structure"))
  (bind _returnvalue (`GameplayStatics.GetPlayerController` 0))
  (bind _returnvalue_x (`KismetMathLibrary.BreakVector` (`self.K2_GetActorLocation`)))
  (bind _returnvalue_2 (`GameplayStatics.GetPlayerPawn` 0))
  (:`Pressed`
    (`self.DisableInput` (stale `self.ReceiveActorBeginOverlap` _asplayer_character) (`GameplayStatics.GetPlayerController` 0))
    (`self.DisableInput` (`GameplayStatics.GetPlayerPawn` 0) (`GameplayStatics.GetPlayerController` 0))
    (bind _returnvalue_x_2 (`KismetMathLibrary.BreakVector` (`self.K2_GetActorLocation` (stale `self.ReceiveActorBeginOverlap` _asplayer_character))))
    (if (> _returnvalue_x_2 _returnvalue_x)
      (bind _widget (`self.CreateWidget`))
      (bind (_direction _opac) (`Timeline|Right` :!via `PlayFromStart`)
        (:`Update`
          (`self.SetOpacRight` _widget _opac))
        (:`Finished`
          (`self.EnableInput` _returnvalue_2 _returnvalue)))
      (elif (<= _returnvalue_x_2 _returnvalue_x)
        (bind _widget_2 (`self.CreateWidget`))
        (bind (_direction_2 _opac_2) (`Timeline|Left` :!via `PlayFromStart`)
          (:`Update`
            (`self.SetOpacLeft` _widget_2 _opac_2))
          (:`Finished`
            (`self.EnableInput` _returnvalue_2 _returnvalue)))))))

(fn `CreateWidget`
  (returns (Widget :type "UserWidget Object Reference"))
  (bind _returnvalue (`|CreateWidget` "/Game/Widgets/BlackScreen.BlackScreen_C"))
  (`UserWidget.AddToViewport` _returnvalue 0)
  (return _returnvalue))

(fn `SetOpacLeft`
  (params (Widget :type "UserWidget Object Reference") (Opacity :type "Float (double-precision)"))
  (`UserWidget.SetColorAndOpacity` Widget (make `LinearColor` 0.0 0.0 0.0 Opacity)))

(fn `SetOpacRight`
  (params (Widget :type "UserWidget Object Reference") (Opacity :type "Float (double-precision)"))
  (`UserWidget.SetColorAndOpacity` Widget (make `LinearColor` 0.0 0.0 0.0 Opacity)))

(fn `UserConstructionScript`)