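; Talkable character that lets an overlapping PlayerCharacter press E to open a SpeakingWindow widget and pause them.
; While the window is opening, Tick glides the player via FInterpTo to the nearest of four anchor points (Back, Front, Left, Right) until they arrive.
; Left/right approaches also rotate the player's flipbook based on which side of the character they stand.
; Releasing E closes the window and unpauses after a five-second delay.
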(event `self.ReceiveTick`
  (params (DeltaSeconds :type "Float (single-precision)"))
  (`self.SetLocation` (stale `self.ReceiveActorBeginOverlap` OtherActor) (`self.SetLoc`)))

(event `self.ReceiveActorBeginOverlap`
  (params (OtherActor :type "Actor Object Reference"))
  (cast `/Game/PlayerCharacter/PlayerCharacter` OtherActor)
  (`KismetSystemLibrary.PrintString` "Hello")
  (`self.EnableInput` (`GameplayStatics.GetPlayerController` 0)))

(event `self.ReceiveActorEndOverlap`
  (params (OtherActor :type "Actor Object Reference"))
  (cast `/Game/PlayerCharacter/PlayerCharacter` OtherActor)
  (`KismetSystemLibrary.PrintString` "bye")
  (`self.DisableInput` (`GameplayStatics.GetPlayerController` 0)))

(event `Key|E`
  (params (Key :type "Key Structure"))
  (:`Pressed`
    (if (not (`self.WidgetSpawned`))
      (bind _asplayer_character (cast `/Game/PlayerCharacter/PlayerCharacter` (stale `self.ReceiveActorBeginOverlap` OtherActor)))
      (set `self.WidgetSpawned` true)
      (set `self.SetLoc` true)
      (set `/Game/PlayerCharacter/PlayerCharacter.InPause?` true _asplayer_character)
      (bind _returnvalue (`|CreateWidget` "/Game/Widgets/SpeakingWindow.SpeakingWindow_C"))
      (`UserWidget.SetAlignmentInViewport` _returnvalue (0.0 0.0))
      (bind _output_get (set `self.UiWidget` _returnvalue))
      (`UserWidget.AddToViewport` _output_get 0)))
  (:`Released`
    (`KismetSystemLibrary.Delay` 5.0)
    (`Widget.RemoveFromParent` (`self.UiWidget`))
    (set `self.WidgetSpawned` false)
    (set `self.SetLoc` false)
    (bind _asplayer_character_2 (cast `/Game/PlayerCharacter/PlayerCharacter` (stale `self.ReceiveActorBeginOverlap` OtherActor)))
    (set `/Game/PlayerCharacter/PlayerCharacter.InPause?` false _asplayer_character_2)))

(fn `IsCloserToBack`
  (params (Player :type "Actor Object Reference"))
  (returns (IsCloserToBack :type Boolean))
  (bind _returnvalue (`self.K2_GetActorLocation` Player))
  (bind _returnvalue_2 (`KismetMathLibrary.Vector_Distance` _returnvalue (`SceneComponent.K2_GetComponentLocation` (`self.back`))))
  (return (and (<= _returnvalue_2 (`KismetMathLibrary.Vector_Distance` _returnvalue (`SceneComponent.K2_GetComponentLocation` (`self.front`)))) (<= _returnvalue_2 (`KismetMathLibrary.Vector_Distance` _returnvalue (`SceneComponent.K2_GetComponentLocation` (`self.right`)))) (<= _returnvalue_2 (`KismetMathLibrary.Vector_Distance` _returnvalue (`SceneComponent.K2_GetComponentLocation` (`self.left`)))) (not (== (`self.K2_GetActorLocation` Player) (`SceneComponent.K2_GetComponentLocation` (`self.back`)) :`ErrorTolerance` (`self.ErrorTolerance`))))))

(fn `IsCloserToFront`
  (params (Player :type "Actor Object Reference"))
  (returns (IsCloserToFront :type Boolean))
  (bind _returnvalue (`self.K2_GetActorLocation` Player))
  (bind _returnvalue_2 (`KismetMathLibrary.Vector_Distance` _returnvalue (`SceneComponent.K2_GetComponentLocation` (`self.front`))))
  (return (and (< _returnvalue_2 (`KismetMathLibrary.Vector_Distance` _returnvalue (`SceneComponent.K2_GetComponentLocation` (`self.back`)))) (< _returnvalue_2 (`KismetMathLibrary.Vector_Distance` _returnvalue (`SceneComponent.K2_GetComponentLocation` (`self.right`)))) (< _returnvalue_2 (`KismetMathLibrary.Vector_Distance` _returnvalue (`SceneComponent.K2_GetComponentLocation` (`self.left`)))) (not (== (`self.K2_GetActorLocation` Player) (`SceneComponent.K2_GetComponentLocation` (`self.front`)) :`ErrorTolerance` (`self.ErrorTolerance`))))))

(fn `IsCloserToLeft`
  (params (Player :type "Actor Object Reference"))
  (returns (IsCloserToLeft :type Boolean))
  (bind _returnvalue (`self.K2_GetActorLocation` Player))
  (bind _returnvalue_2 (`KismetMathLibrary.Vector_Distance` _returnvalue (`SceneComponent.K2_GetComponentLocation` (`self.left`))))
  (return (and (<= _returnvalue_2 (`KismetMathLibrary.Vector_Distance` _returnvalue (`SceneComponent.K2_GetComponentLocation` (`self.back`)))) (<= _returnvalue_2 (`KismetMathLibrary.Vector_Distance` _returnvalue (`SceneComponent.K2_GetComponentLocation` (`self.front`)))) (<= _returnvalue_2 (`KismetMathLibrary.Vector_Distance` _returnvalue (`SceneComponent.K2_GetComponentLocation` (`self.right`)))) (not (== (`self.K2_GetActorLocation` Player) (`SceneComponent.K2_GetComponentLocation` (`self.left`)) :`ErrorTolerance` (`self.ErrorTolerance`))))))

(fn `IsCloserToRight`
  (params (Player :type "Actor Object Reference"))
  (returns (IsCloserToRight :type Boolean))
  (bind _returnvalue (`self.K2_GetActorLocation` Player))
  (bind _returnvalue_2 (`KismetMathLibrary.Vector_Distance` _returnvalue (`SceneComponent.K2_GetComponentLocation` (`self.right`))))
  (return (and (< _returnvalue_2 (`KismetMathLibrary.Vector_Distance` _returnvalue (`SceneComponent.K2_GetComponentLocation` (`self.front`)))) (< _returnvalue_2 (`KismetMathLibrary.Vector_Distance` _returnvalue (`SceneComponent.K2_GetComponentLocation` (`self.back`)))) (< _returnvalue_2 (`KismetMathLibrary.Vector_Distance` _returnvalue (`SceneComponent.K2_GetComponentLocation` (`self.left`)))) (not (== (`self.K2_GetActorLocation` Player) (`SceneComponent.K2_GetComponentLocation` (`self.right`)) :`ErrorTolerance` (`self.ErrorTolerance`))))))

(fn `IsOnBackSide`
  (params (Player :type "Actor Object Reference"))
  (returns (`IsOnBackSide?` :type Boolean))
  (return (== (`self.K2_GetActorLocation` Player) (`SceneComponent.K2_GetComponentLocation` (`self.back`)) :`ErrorTolerance` (`self.ErrorTolerance`))))

(fn `IsOnFrontSide`
  (params (Player :type "Actor Object Reference"))
  (returns (`IsOnFrontSide?` :type Boolean))
  (return (== (`self.K2_GetActorLocation` Player) (`SceneComponent.K2_GetComponentLocation` (`self.front`)) :`ErrorTolerance` (`self.ErrorTolerance`))))

(fn `IsOnLeft`
  (params (Player :type "Actor Object Reference"))
  (returns (OnLeft :type Boolean))
  (bind _returnvalue_x (`KismetMathLibrary.BreakVector` (`self.K2_GetActorLocation`)))
  (bind _asplayer_character (cast `/Game/PlayerCharacter/PlayerCharacter` Player))
  (bind _returnvalue_x_2 (`KismetMathLibrary.BreakVector` (`self.K2_GetActorLocation` _asplayer_character)))
  (return (< _returnvalue_x_2 _returnvalue_x)))

(fn `IsOnLeftSide`
  (params (Player :type "Actor Object Reference"))
  (returns (`IsOnLeftSide?` :type Boolean))
  (return (== (`self.K2_GetActorLocation` Player) (`SceneComponent.K2_GetComponentLocation` (`self.left`)) :`ErrorTolerance` (`self.ErrorTolerance`))))

(fn `IsOnRight`
  (params (Player :type "Actor Object Reference"))
  (returns (OnRight :type Boolean))
  (bind _returnvalue_x (`KismetMathLibrary.BreakVector` (`self.K2_GetActorLocation`)))
  (bind _asplayer_character (cast `/Game/PlayerCharacter/PlayerCharacter` Player))
  (bind _returnvalue_x_2 (`KismetMathLibrary.BreakVector` (`self.K2_GetActorLocation` _asplayer_character)))
  (return (>= _returnvalue_x_2 _returnvalue_x)))

(fn `IsOnRightSide`
  (params (Player :type "Actor Object Reference"))
  (returns (`IsOnRightSide?` :type Boolean))
  (return (== (`self.K2_GetActorLocation` Player) (`SceneComponent.K2_GetComponentLocation` (`self.right`)) :`ErrorTolerance` (`self.ErrorTolerance`))))

(fn `LeftRotationWhenToClose`
  (params (Player :type "Actor Object Reference"))
  (bind _asplayer_character (cast `/Game/PlayerCharacter/PlayerCharacter` Player))
  (`SceneComponent.K2_SetWorldRotation` (`/Game/PlayerCharacter/PlayerCharacter.PaperFlipbook` _asplayer_character) (struct :`Roll` -45.0) false false))

(fn `RightRotationWhenToClose`
  (params (Player :type "Actor Object Reference"))
  (bind _asplayer_character (cast `/Game/PlayerCharacter/PlayerCharacter` Player))
  (`SceneComponent.K2_SetWorldRotation` (`/Game/PlayerCharacter/PlayerCharacter.PaperFlipbook` _asplayer_character) (struct :`Yaw` 180.0 :`Roll` 45.0) false false))

(fn `SetLocation`
  (params (Player :type "Actor Object Reference") (`SetLocation?` :type Boolean))
  (bind _asplayer_character (cast `/Game/PlayerCharacter/PlayerCharacter` Player))
  (if `SetLocation?`
    (bind _isclosertoback (`self.IsCloserToBack` _asplayer_character))
    (if _isclosertoback
      (`self.SetLocationBack` _isclosertoback _asplayer_character)
      (else
        (bind _isclosertofront (`self.IsCloserToFront` _asplayer_character))
        (if _isclosertofront
          (`self.SetLocationFront` _isclosertofront _asplayer_character)
          (else
            (bind _isclosertoleft (`self.IsCloserToLeft` _asplayer_character))
            (if _isclosertoleft
              (`self.SetLocationLeft` _isclosertoleft _asplayer_character)
              (else
                (bind _isclosertoright (`self.IsCloserToRight` _asplayer_character))
                (if _isclosertoright
                  (`self.SetLocationRight` _isclosertoright _asplayer_character)
                  (else
                    (set `self.SetLoc` false)))))
            (`self.SetRotationHorizontal` _asplayer_character)))))))

(fn `SetLocationBack`
  (params (`Back?` :type Boolean) (Player :type "Actor Object Reference"))
  (bind (_returnvalue_x _returnvalue_y _returnvalue_z) (`KismetMathLibrary.BreakVector` (`self.K2_GetActorLocation` Player)))
  (bind _returnvalue (`GameplayStatics.GetWorldDeltaSeconds`))
  (bind (_returnvalue_x_2 _returnvalue_y_2) (`KismetMathLibrary.BreakVector` (`SceneComponent.K2_GetComponentLocation` (`self.back`))))
  (if `Back?`
    (`self.K2_SetActorLocation` Player (`KismetMathLibrary.MakeVector` (`KismetMathLibrary.FInterpTo` _returnvalue_x _returnvalue_x_2 _returnvalue 3.0) (`KismetMathLibrary.FInterpTo` _returnvalue_y _returnvalue_y_2 _returnvalue 3.0) _returnvalue_z) true false)
    (if (`self.IsOnBackSide` Player)
      (set `self.SetLoc` false))))

(fn `SetLocationFront`
  (params (`Front?` :type Boolean) (Player :type "Actor Object Reference"))
  (bind (_returnvalue_x _returnvalue_y _returnvalue_z) (`KismetMathLibrary.BreakVector` (`self.K2_GetActorLocation` Player)))
  (bind _returnvalue (`GameplayStatics.GetWorldDeltaSeconds`))
  (bind (_returnvalue_x_2 _returnvalue_y_2) (`KismetMathLibrary.BreakVector` (`SceneComponent.K2_GetComponentLocation` (`self.front`))))
  (if `Front?`
    (`self.K2_SetActorLocation` Player (`KismetMathLibrary.MakeVector` (`KismetMathLibrary.FInterpTo` _returnvalue_x _returnvalue_x_2 _returnvalue 3.0) (`KismetMathLibrary.FInterpTo` _returnvalue_y _returnvalue_y_2 _returnvalue 3.0) _returnvalue_z) true false)
    (if (`self.IsOnFrontSide` Player)
      (set `self.SetLoc` false))))

(fn `SetLocationLeft`
  (params (`Left?` :type Boolean) (Player :type "Actor Object Reference"))
  (bind _returnvalue (`GameplayStatics.GetWorldDeltaSeconds`))
  (bind (_returnvalue_x _returnvalue_y _returnvalue_z) (`KismetMathLibrary.BreakVector` (`self.K2_GetActorLocation` Player)))
  (bind (_returnvalue_x_2 _returnvalue_y_2) (`KismetMathLibrary.BreakVector` (`SceneComponent.K2_GetComponentLocation` (`self.left`))))
  (if `Left?`
    (`self.K2_SetActorLocation` Player (`KismetMathLibrary.MakeVector` (`KismetMathLibrary.FInterpTo` _returnvalue_x _returnvalue_x_2 _returnvalue 3.0) (`KismetMathLibrary.FInterpTo` _returnvalue_y _returnvalue_y_2 _returnvalue 3.0) _returnvalue_z) true false)
    (if (`self.IsOnLeftSide` Player)
      (`KismetSystemLibrary.PrintString` "Hello")
      (set `self.SetLoc` false))))

(fn `SetLocationRight`
  (params (`Right?` :type Boolean) (Player :type "Actor Object Reference"))
  (bind (_returnvalue_x _returnvalue_y _returnvalue_z) (`KismetMathLibrary.BreakVector` (`self.K2_GetActorLocation` Player)))
  (bind _returnvalue (`GameplayStatics.GetWorldDeltaSeconds`))
  (bind (_returnvalue_x_2 _returnvalue_y_2) (`KismetMathLibrary.BreakVector` (`SceneComponent.K2_GetComponentLocation` (`self.right`))))
  (if `Right?`
    (`self.K2_SetActorLocation` Player (`KismetMathLibrary.MakeVector` (`KismetMathLibrary.FInterpTo` _returnvalue_x _returnvalue_x_2 _returnvalue 3.0) (`KismetMathLibrary.FInterpTo` _returnvalue_y _returnvalue_y_2 _returnvalue 3.0) _returnvalue_z) true false)
    (if (`self.IsOnRightSide` Player)
      (set `self.SetLoc` false))))

(fn `SetRotationHorizontal`
  (params (Player :type "Actor Object Reference"))
  (if (`self.IsOnRight` Player)
    (`self.RightRotationWhenToClose` Player)
    (elif (`self.IsOnLeft` Player)
      (`self.LeftRotationWhenToClose` Player))))

(fn `UserConstructionScript`)