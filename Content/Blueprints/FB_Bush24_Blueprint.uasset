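; Bush actor Blueprint that the player can harvest for food by pressing P while overlapping it.
; Overlap begin caches the PlayerCharacter and enables input on the bush for player 0, and overlap end disables it.
; On P, if the character has Pesoc set and HasMedved clear, it sets HasFood and destroys the bush.
; Otherwise it prints "put down medved", whichever condition failed.
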(event `self.ReceiveActorBeginOverlap`
  (params (OtherActor :type "Actor Object Reference"))
  (bind _asplayer_character (cast `/Game/PlayerCharacter/PlayerCharacter` OtherActor))
  (`self.EnableInput` (`GameplayStatics.GetPlayerController` 0)))

(event `self.ReceiveActorEndOverlap`
  (params (OtherActor :type "Actor Object Reference"))
  (cast `/Game/PlayerCharacter/PlayerCharacter` OtherActor)
  (`self.DisableInput` (`GameplayStatics.GetPlayerController` 0)))

(event `Key|P`
  (params (Key :type "Key Structure"))
  (:`Pressed`
    (if (and (`/Game/PlayerCharacter/PlayerCharacter.Pesoc` (stale `self.ReceiveActorBeginOverlap` _asplayer_character)) (not (`/Game/PlayerCharacter/PlayerCharacter.HasMedved` (stale `self.ReceiveActorBeginOverlap` _asplayer_character))))
      (set `/Game/PlayerCharacter/PlayerCharacter.HasFood` true (stale `self.ReceiveActorBeginOverlap` _asplayer_character))
      (`self.K2_DestroyActor`)
      (else
        (`KismetSystemLibrary.PrintString` "put down medved")))))

(fn `UserConstructionScript`)