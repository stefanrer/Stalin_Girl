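; ScreenShot captures a screenshot for the current save file when play begins.
; On BeginPlay it gets CurrentSaveFile from the 25D game mode and builds a HighResShot console command that uses it as the filename.
; It then loads that slot's GameSave and saves it back without changes.
; A WasInMenu check is left disconnected, so the capture is not gated by it.
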(event `self.ReceiveBeginPlay`
  (bind _as25d (cast `/Game/Gamemode/25D` (`GameplayStatics.GetGameMode`)))
  (bind _currentsavefile (`/Game/Gamemode/25D.CurrentSaveFile` _as25d))
  (`KismetSystemLibrary.ExecuteConsoleCommand` (`KismetStringLibrary.Concat_StrStr` "HighResShot " " " "400x400" " " (`KismetStringLibrary.Concat_StrStr` "filename=" _currentsavefile)) (`GameplayStatics.GetPlayerController` 0))
  (bind _returnvalue (`GameplayStatics.LoadGameFromSlot` _currentsavefile))
  (bind _asgame_save (cast `/Game/SaveFile/GameSave` _returnvalue))
  (`GameplayStatics.SaveGameToSlot` _asgame_save _currentsavefile))

(fn `UserConstructionScript`)